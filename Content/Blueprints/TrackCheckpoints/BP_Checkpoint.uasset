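; BP_Checkpoint is a track checkpoint actor that reports kart crossings to the core game mode for lap tracking.
; When its collision component is overlapped, it reads the kart's last checkpoint ID.
; Crossing checkpoint zero with a last ID of at least three calls CompleteLap on BP_GM_Core; otherwise it calls PassCheckpoint.
; The lap threshold is hard-coded, and all progress handling is delegated to the game mode.
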(event `self.CollisionComponent.OnComponentBeginOverlap`
  (params (OverlappedComponent :type "PrimitiveComponent Object Reference") (OtherActor :type "Actor Object Reference") (OtherComp :type "PrimitiveComponent Object Reference") (OtherBodyIndex :type Integer) (bFromSweep :type Boolean) (SweepResult :type "HitResult Structure (by ref)"))
  (bind _asbp_core_kart (cast `/Game/Blueprints/Gamemodes/Core/BP_Core_Kart` OtherActor :!pure true))
  (bind _asbp_gm_core (cast `/Game/Blueprints/Gamemodes/Core/BP_GM_Core` (`GameplayStatics.GetGameMode`) :!pure true))
  (if (and (>= (`/Game/Blueprints/TrackCheckpoints/BP_Checkpoint.CheckpointID` (`/Game/Blueprints/Gamemodes/Core/BP_Core_Kart.LastCheckpoint` _asbp_core_kart)) 3) (== (`self.CheckpointID`) 0))
    (`/Game/Blueprints/Gamemodes/Core/BP_GM_Core.CompleteLap` _asbp_gm_core _asbp_core_kart self)
    (else
      (`/Game/Blueprints/Gamemodes/Core/BP_GM_Core.PassCheckpoint` _asbp_gm_core OtherActor self))))

(fn `UserConstructionScript`)