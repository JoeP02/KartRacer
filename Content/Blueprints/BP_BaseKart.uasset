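; Base kart Blueprint that simulates a physics-driven vehicle with raycast suspension on four corner points.
; Each tick it traces down from every suspension point and, on a hit, applies impulses to Body at that point.
; CalculateSuspension uses a damped spring along the point's up vector, while CalculateSteering counters sideways velocity to model tyre grip.
; The file contains no input, acceleration or braking logic.
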(event `self.ReceiveBeginPlay`
  (`self.GetSuspensionPoints`))

(event `self.ReceiveTick`
  (params (DeltaSeconds :type "Float (single-precision)"))
  (`self.UpdateCarPhysics`))

(fn `CalculateSteering`
  (params (Hit :type "HitResult Structure") (SuspensionPoint :type "ArrowComponent Object Reference"))
  (locals (SteeringDirection :type "Vector Structure") (SuspensionPointWorldVelocity :type "Vector Structure") (SteeringVelocity :type "Float (double-precision)") (DesiredVelocityChange :type "Float (double-precision)") (DesiredAcceleration :type "Float (double-precision)"))
  (set `local.SteeringDirection` (`SceneComponent.GetRightVector` SuspensionPoint))
  (set `local.SuspensionPointWorldVelocity` (`SceneComponent.GetComponentVelocity` (`local.SuspensionPoint`)))
  (set `local.SteeringVelocity` (`KismetMathLibrary.Dot_VectorVector` (`local.SteeringDirection`) (`local.SuspensionPointWorldVelocity`)))
  (bind _output_get (set `local.DesiredVelocityChange` (* (* (`local.SteeringVelocity`) -1.0) (`self.TyreGripFactor`))))
  (set `local.DesiredAcceleration` (/ _output_get (`GameplayStatics.GetWorldDeltaSeconds`)))
  (`PrimitiveComponent.AddImpulseAtLocation` (`self.Body`) (* (`local.SteeringDirection`) (`self.TyreMass`) (`local.DesiredAcceleration`)) (`SceneComponent.K2_GetComponentLocation` (`local.SuspensionPoint`)) "None"))

(fn `CalculateSuspension`
  (params (Hit :type "HitResult Structure") (SuspensionPoint :type "ArrowComponent Object Reference"))
  (locals (SpringDirection :type "Vector Structure") (SuspensionPointWorldVelocity :type "Vector Structure") (Offset :type "Float (double-precision)") (Velocity :type "Float (double-precision)") (Force :type "Float (double-precision)"))
  (set `local.SpringDirection` (`SceneComponent.GetUpVector` (`local.SuspensionPoint`)))
  (set `local.SuspensionPointWorldVelocity` (`SceneComponent.GetComponentVelocity` (`local.SuspensionPoint`)))
  (set `local.Offset` (- (`self.SuspensionLength`) (`.Distance` (`GameplayStatics.BreakHitResult` Hit))))
  (set `local.Velocity` (`KismetMathLibrary.Dot_VectorVector` (`local.SpringDirection`) (`local.SuspensionPointWorldVelocity`)))
  (set `local.Force` (- (* (`local.Offset`) (`self.SpringStrength`)) (* (`local.Velocity`) (`self.SuspensionDamping`))))
  (`PrimitiveComponent.AddImpulseAtLocation` (`self.Body`) (* (`local.SpringDirection`) (`local.Force`)) (`SceneComponent.K2_GetComponentLocation` (`local.SuspensionPoint`)) "None"))

(fn `GetSuspensionPoints`
  (bind _suspensionpoints (`self.SuspensionPoints`))
  (`KismetArrayLibrary.Array_Clear` _suspensionpoints)
  (`KismetArrayLibrary.Array_Add` _suspensionpoints (`self.FL_Suspension`))
  (`KismetArrayLibrary.Array_Add` _suspensionpoints (`self.FR_Suspension`))
  (`KismetArrayLibrary.Array_Add` _suspensionpoints (`self.RR_Suspension`))
  (`KismetArrayLibrary.Array_Add` _suspensionpoints (`self.RL_Suspension`)))

(fn `UpdateCarPhysics`
  (for _array_element (`self.SuspensionPoints`)
    (bind _returnvalue (`SceneComponent.K2_GetComponentLocation` _array_element))
    (bind (_outhit _returnvalue_2) (`KismetSystemLibrary.LineTraceSingle` :`Start` _returnvalue :`End` (+ _returnvalue (* (* (`KismetMathLibrary.GetUpVector` (`SceneComponent.K2_GetComponentRotation` _array_element)) (`self.SuspensionLength`)) -1.0)) :`TraceChannel` "TraceTypeQuery1" :`DrawDebugType` "ForOneFrame"))
    (if _returnvalue_2
      (`self.CalculateSuspension` _outhit _array_element)
      (`self.CalculateSteering` _outhit _array_element))))

(fn `UserConstructionScript`)