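; Base kart Blueprint built around a CarBall component, with only its motion-sampling step implemented.
; UpdateSphere projects the ball's velocity onto the actor's forward and right vectors to store ForwardSpeed and LateralSpeed.
; It then runs a sphere trace on the Visibility channel, whose result is unused.
; The event graph and construction script are empty, and nothing in this file calls UpdateSphere.
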(fn `UpdateSphere`
  (locals (ForwardSpeed :type "Float (double-precision)") (LateralSpeed :type "Float (double-precision)"))
  (set `local.ForwardSpeed` (`KismetMathLibrary.Dot_VectorVector` (`SceneComponent.GetComponentVelocity` (`self.CarBall`)) (`self.GetActorForwardVector`)))
  (set `local.LateralSpeed` (`KismetMathLibrary.Dot_VectorVector` (`SceneComponent.GetComponentVelocity` (`self.CarBall`)) (`self.GetActorRightVector`)))
  (`KismetSystemLibrary.SphereTraceSingle` (0.0 0.0 0.0) (0.0 0.0 0.0) 0.0 "TraceTypeQuery1"))

(fn `UserConstructionScript`)