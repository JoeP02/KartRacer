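; BP_PC_GameInit is the player controller for game initialization, showing the login screen and routing the login result.
; On BeginPlay it binds to the KartRacingOnlineSubsystem login-completed event and, for the local controller, creates WBP_GameInit and adds it to the viewport.
; A successful login opens the MainMenu level, while a failure passes the error to the login widget.
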(event `self.ReceiveBeginPlay`
  (add `KartRacingOnlineSubsystem.OnKartLoginCompleted` (subsystem `KartRacingOnlineSubsystem`) (delegate `OnLoginCompletes`))
  (if (`self.IsLocalPlayerController`)
    (bind _returnvalue (`|CreateWidget` "/Game/Widgets/GameInit/WBP_GameInit.WBP_GameInit_C"))
    (bind _output_get (set `self.LoginScreen` _returnvalue))
    (`UserWidget.AddToViewport` _output_get 0)))

(event `OnLoginCompletes`
  (params (LocalUserNum :type Integer) (bWasSuccessful :type Boolean) (Error :type String))
  (if bWasSuccessful
    (`GameplayStatics.OpenLevelBySoftObjectPtr` "/Game/Maps/MainMenu.MainMenu")
    (else
      (`/Game/Widgets/GameInit/WBP_GameInit.ErrorFromLogin` (`self.LoginScreen`) Error))))

(fn `UserConstructionScript`)