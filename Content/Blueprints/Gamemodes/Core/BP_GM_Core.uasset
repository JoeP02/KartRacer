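; Core game mode for a kart game that handles player spawn placement and kart skins.
; ChoosePlayerStart gives each player a free PlayerStart by tagging chosen ones "Used" so spawns do not overlap.
; On player restart, the controlled BP_Core_Kart gets the next material from KartMaterials through an incrementing SkinCount.
; The PassCheckpoint event only prints the kart name and checkpoint ID.
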(event `self.K2_OnRestartPlayer`
  (params (NewPlayer :type "Controller Object Reference"))
  (bind _asbp_core_kart (cast `/Game/Blueprints/Gamemodes/Core/BP_Core_Kart` (`Controller.K2_GetPawn` NewPlayer)))
  (set `/Game/Blueprints/Gamemodes/Core/BP_Core_Kart.KartMaterial` (`|GetArrayItem` (`self.KartMaterials`) (`self.SkinCount`)) _asbp_core_kart)
  (`/Engine/EditorBlueprintResources/StandardMacros.IncrementInt` (`self.SkinCount`)))

(event `PassCheckpoint`
  (params (Player :type "Actor Object Reference") (CheckpointID :type Integer))
  (`KismetSystemLibrary.PrintString` (`KismetStringLibrary.Concat_StrStr` "Kart " (`KismetSystemLibrary.GetDisplayName` Player) " Passed Through Checkpoint with ID " (`KismetStringLibrary.Conv_IntToString` CheckpointID))))

(fn `ChoosePlayerStart`
  (params (Player :type "Controller Object Reference"))
  (returns (ReturnValue :type "Actor Object Reference"))
  ;[1 1 1] Makes sure each player is at their own start point. Without this multiple players could spawn at the same player start location. This uses the player start tag system so when one is already take it will assign it the used tag so that when another player joins the game mode wont pick that location for them to spawn.
  (bind _outactors (`GameplayStatics.GetAllActorsOfClass` "/Script/Engine.PlayerStart"))
  (for _array_element _outactors
    (if (!= (`PlayerStart.PlayerStartTag` _array_element) "Used")
      (set `PlayerStart.PlayerStartTag` "Used" _array_element)
      (return _array_element))))

(fn `UserConstructionScript`)