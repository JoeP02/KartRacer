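; Player kart actor that drives by pushing a physics Ball along the actor's forward vector.
; Input events set forward force and steering locally, then send them to server events that reject magnitudes above 1, although forward input is pre-scaled far higher.
; Tick applies the force, yaws the actor and KartMesh by steering over minimum turning radius, and draws an upward debug trace whose result is unused.
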(event `self.ReceiveTick`
  (params (DeltaSeconds :type "Float (single-precision)"))
  (bind _returnvalue (`self.K2_GetActorLocation`))
  (bind _returnvalue_2 (* (/ (* 1.0 (`GameplayStatics.GetWorldDeltaSeconds`)) (`self.MinimunTurningRadius`)) (`self.SteeringInput`)))
  (`|ExecutionSequence`
    (:`then_0`
      (if (> (`KismetMathLibrary.Abs` (`self.ForwardInput`)) 0.0)
        (`PrimitiveComponent.AddForce` (`self.Ball`) (* (`self.GetActorForwardVector`) (`self.ForwardInput`)) "None" false)))
    (:`then_1`
      (`KismetSystemLibrary.LineTraceSingle` :`Start` _returnvalue :`End` (+ _returnvalue (* (`self.GetActorUpVector`) 200.0)) :`TraceChannel` "TraceTypeQuery1" :`DrawDebugType` "ForOneFrame")
      (`self.K2_AddActorLocalRotation` (`KismetMathLibrary.RotatorFromAxisAndAngle` (`self.GetActorUpVector`) _returnvalue_2))
      (`SceneComponent.K2_AddRelativeRotation` (`self.KartMesh`) (`KismetMathLibrary.MakeRotator` 0.0 0.0 _returnvalue_2) false false))))

(event `MoveKartInput`
  (params (Value :type "Float (double-precision)"))
  ;[1 1 1] Inputs and Handled by updating the clients first then telling the server about the change
  (bind _output_get (set `self.ForwardInput` (`KismetMathLibrary.SelectFloat` (* Value (`self.ForwardAcceleration`) 100000.0) (* Value (`self.BackwardsAcceleration`) 100000.0) (> Value 0.0))))
  (`self.Server_MoveKartInput` _output_get))

(event `Server_MoveKartInput`
  (params (Value :type "Float (double-precision)"))
  ;[1 1 1] Inputs and Handled by updating the clients first then telling the server about the change
  ;;[1 1 1] Moving - Sets the Input Value From The User
  (if (<= (`KismetMathLibrary.Abs` Value) 1.0)
    (set `self.ForwardInput` Value)
    (else
      (`KismetSystemLibrary.PrintString` "Input Valodation Error"))))

(event `TurnKartInput`
  (params (Value :type "Float (double-precision)"))
  ;[1 1 1] Inputs and Handled by updating the clients first then telling the server about the change
  (bind _output_get (set `self.SteeringInput` Value))
  (`self.Server_TurnKartInput` _output_get))

(event `Server_TurnKartInput`
  (params (Value :type "Float (double-precision)"))
  ;[1 1 1] Inputs and Handled by updating the clients first then telling the server about the change
  ;;[1 1 1] Turning - Sets the Input Value From The User
  (if (<= (`KismetMathLibrary.Abs` Value) 1.0)
    (set `self.SteeringInput` Value)
    (else
      (`KismetSystemLibrary.PrintString` "Input Validation Error"))))

(fn `UserConstructionScript`)