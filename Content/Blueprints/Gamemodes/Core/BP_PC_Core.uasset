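; BP_PC_Core is the player controller that routes Enhanced Input to the player's kart.
; On BeginPlay it adds the IMC_Kart mapping context for local players and caches the controlled pawn as a BP_Core_Kart, with both steps skipped for non-local controllers.
; Forward and turn actions pass their values to the kart's MoveKartInput and TurnKartInput on both Triggered and Completed.
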(event `self.ReceiveBeginPlay`
  (if (`self.IsLocalPlayerController`)
    (`EnhancedInputSubsystemInterface.AddMappingContext` (subsystem `EnhancedInputLocalPlayerSubsystem`) "/Game/Input/Kart/IMC_Kart.IMC_Kart" 0 (struct)))
  (bind _asbp_core_kart (cast `/Game/Blueprints/Gamemodes/Core/BP_Core_Kart` (`self.K2_GetPawn`)))
  (set `self.PlayerKart` _asbp_core_kart))

(event `EnhancedInput|/Game/Input/Kart/IA_KartForward`
  (params (ActionValue :type "Float (double-precision)") (ElapsedSeconds :type "Float (double-precision)") (TriggeredSeconds :type "Float (double-precision)") (InputAction :type "InputAction Object Reference" :default "/Game/Input/Kart/IA_KartForward.IA_KartForward"))
  (:`Triggered`
    (`/Game/Blueprints/Gamemodes/Core/BP_Core_Kart.MoveKartInput` (`self.PlayerKart`) ActionValue :!label _label))
  (:`Completed`
    (goto _label)))

(event `EnhancedInput|/Game/Input/Kart/IA_KartTurn`
  (params (ActionValue :type "Float (double-precision)") (ElapsedSeconds :type "Float (double-precision)") (TriggeredSeconds :type "Float (double-precision)") (InputAction :type "InputAction Object Reference" :default "/Game/Input/Kart/IA_KartTurn.IA_KartTurn"))
  (:`Triggered`
    (`/Game/Blueprints/Gamemodes/Core/BP_Core_Kart.TurnKartInput` (`self.PlayerKart`) ActionValue :!label _label_2))
  (:`Completed`
    (goto _label_2)))

(fn `UserConstructionScript`)