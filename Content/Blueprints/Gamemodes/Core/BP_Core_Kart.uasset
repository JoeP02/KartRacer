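; Core kart that drives with hand-written vehicle physics instead of a movement component.
; Each Tick turns throttle, quadratic air drag and rolling resistance into acceleration and velocity.
; Steering rotates velocity and actor by distance travelled over turning radius, then a swept offset moves the kart, zeroing velocity on blocking hits.
; Input is applied locally and sent to server events that range-check it.
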(event `self.ReceiveBeginPlay`)

(event `self.ReceiveTick`
  (params (DeltaSeconds :type "Float (single-precision)"))
  ;[1 1 1] Acceleration = Force / Mass
  (bind _output_get (set `self.Force` (* (`self.GetActorForwardVector`) (`self.MaxForwardForce`) (`self.ForwardInput`))))
  (bind _output_get_2 (set `self.Force` (+ _output_get (`self.CalculateAirResistance`) (`self.CalculateRollingResistance`))))
  (bind _output_get_3 (set `self.Acceleration` (/ _output_get_2 (`self.KartMass`))))
  ;[1 1 1] Velocity = Velocity + Acceleration * Time
  (set `self.Velocity` (+ (* _output_get_3 (`GameplayStatics.GetWorldDeltaSeconds`)) (`self.Velocity`)))
  (`self.ApplyRotation`)
  (`self.UpdateLocationFromVelocity`))

(event `Server_MoveKartInput`
  (params (Value :type "Float (double-precision)"))
  ;[1 1 1] Moving - Sets the Input Value From The User
  (if (<= (`KismetMathLibrary.Abs` Value) 1.0)
    (set `self.ForwardInput` Value)
    (else
      (`KismetSystemLibrary.PrintString` "Input Valodation Error"))))

(event `MoveKartInput`
  (params (Value :type "Float (double-precision)"))
  (bind _output_get (set `self.ForwardInput` Value))
  (`self.Server_MoveKartInput` _output_get))

(event `Server_TurnKartInput`
  (params (Value :type "Float (double-precision)"))
  ;[1 1 1] Turning - Sets the Input Value From The User
  (if (<= (`KismetMathLibrary.Abs` Value) 1.0)
    (set `self.SteeringInput` Value)
    (else
      (`KismetSystemLibrary.PrintString` "Input Validation Error"))))

(event `TurnKartInput`
  (params (Value :type "Float (double-precision)"))
  (bind _output_get (set `self.SteeringInput` Value))
  (`self.Server_TurnKartInput` _output_get))

(fn `ApplyRotation`
  (bind _returnvalue (`KismetMathLibrary.RotatorFromAxisAndAngle` (`self.GetActorUpVector`) (* (/ (* (`KismetMathLibrary.Dot_VectorVector` (`self.GetActorForwardVector`) (`self.Velocity`)) (`GameplayStatics.GetWorldDeltaSeconds`)) (`self.MinimunTurningRadius`)) (`self.SteeringInput`))))
  ;[1 1 1] Rotate Around Axis
  (set `self.Velocity` (`KismetMathLibrary.GreaterGreater_VectorRotator` (`self.Velocity`) _returnvalue))
  (`self.K2_AddActorWorldRotation` _returnvalue))

(fn `CalculateAirResistance`
  (returns (AirResistance :type "Vector Structure"))
  (bind _velocity (`self.Velocity`))
  (return (`KismetMathLibrary.NegateVector` (* (`KismetMathLibrary.VSizeSquared` _velocity) (`KismetMathLibrary.Normal` _velocity) (`self.DragCoeficient`)))))

(fn `CalculateRollingResistance`
  (returns (RollingResistance :type "Vector Structure"))
  (return (* (* (`self.KartMass`) -9.8) (`self.RollingResistanceCoefficient`) (`KismetMathLibrary.Normal` (`self.Velocity`)))))

(fn `UpdateLocationFromVelocity`
  ;[1 1 1] Offset = Velocity * 100 (m/s to cm/s) * Time
  (bind _sweephitresult (`self.K2_AddActorWorldOffset` (* (`GameplayStatics.GetWorldDeltaSeconds`) (`self.Velocity`) 100.0) true))
  ;[1 1 1] If Hits Something then Reset Velocity to 0
  (if (`GameplayStatics.BreakHitResult` _sweephitresult)
    (set `self.Velocity` (0.0 0.0 0.0))))

(fn `UserConstructionScript`)