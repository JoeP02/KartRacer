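; BP_Spawner is a server-authoritative spawner that places a configurable pickup actor at its root location and respawns it after it is collected.
; On BeginPlay, SpawnActor runs only with authority, spawning ActorToSpawn and binding to its OnPickedUp event.
; A pickup starts a one-shot PickupCooldown timer, whose completion handler calls SpawnActor again, repeating the cycle without polling on Tick.
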(event `self.ReceiveBeginPlay`
  (`self.SpawnActor`))

(fn `On Picked Up`
  (`KismetSystemLibrary.K2_SetTimerDelegate` (`|CreateDelegate` :!event `Pickup Timer Cooldown Ended`) (`self.PickupCooldown`)))

(fn `Pickup Timer Cooldown Ended`
  (`self.SpawnActor`))

(fn `SpawnActor`
  (`/Engine/EditorBlueprintResources/ActorMacros.Switch Has Authority`
    (:`Authority`
      (bind _returnvalue (`|SpawnActorFromClass` (`self.ActorToSpawn`) (`KismetMathLibrary.MakeTransform` (`SceneComponent.K2_GetComponentLocation` (`self.DefaultSceneRoot`))) "Undefined" "MultiplyWithRoot" null null))
      (add `/Game/Blueprints/Pickups/BP_BasePickup.OnPickedUp` _returnvalue (`|CreateDelegate` :!event `On Picked Up`)))))

(fn `UserConstructionScript`)