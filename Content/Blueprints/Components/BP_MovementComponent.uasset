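; Kart movement component that simulates driving physics on locally controlled karts, gated by network role.
; Tick packs throttle, steering and timing into an FPlayerMove, stores it as LastMove for outside access, and simulates it.
; SimulateMove integrates engine force, air drag and rolling resistance into Velocity, turns by minimum turning radius, then moves the owner with sweep.
; The velocity reset on blocking hits is disconnected and never runs.
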(event `self.ReceiveTick`
  (params (DeltaSeconds :type "Float (single-precision)"))
  (bind _returnvalue (`self.GetOwner`))
  (if (or (`|EnumEquality` (`Actor.GetLocalRole` _returnvalue) "ROLE_AutonomousProxy") (`|EnumEquality` (`Actor.GetRemoteRole` _returnvalue) "ROLE_SimulatedProxy"))
    (bind _output_get (set `self.LastMove` (`self.CreateMove` DeltaSeconds)))
    (`self.SimulateMove` _output_get)))

(fn `ApplyRotation`
  (params (SteeringInput :type "Float (double-precision)") (DeltaTime :type "Float (double-precision)"))
  (bind _returnvalue (`self.GetOwner`))
  (bind _returnvalue_2 (`KismetMathLibrary.RotatorFromAxisAndAngle` (`Actor.GetActorUpVector` _returnvalue) (* SteeringInput (/ (* DeltaTime (`KismetMathLibrary.Dot_VectorVector` (`Actor.GetActorForwardVector` (`self.GetOwner`)) (`self.Velocity`))) (`self.MinimunTurningRadius`)))))
  ;[1 1 1] Rotate Around Axis
  (set `self.Velocity` (`KismetMathLibrary.GreaterGreater_VectorRotator` (`self.Velocity`) _returnvalue_2))
  (`Actor.K2_AddActorWorldRotation` _returnvalue _returnvalue_2 false false))

(fn `CalculateAirResistance`
  (returns (AirResistance :type "Vector Structure"))
  (bind _velocity (`self.Velocity`))
  (return (`KismetMathLibrary.NegateVector` (* (`KismetMathLibrary.VSizeSquared` _velocity) (`KismetMathLibrary.Normal` _velocity) (`self.DragCoeficient`)))))

(fn `CalculateRollingResistance`
  (returns (RollingResistance :type "Vector Structure"))
  (return (* (* (`self.KartMass`) -9.8) (`self.RollingResistanceCoefficient`) (`KismetMathLibrary.Normal` (`self.Velocity`)))))

(fn `CreateMove`
  (params (DeltaTime :type "Float (single-precision)"))
  (returns (FPlayerMove :type "/Game/Blueprints/Gamemodes/Core/FPlayerMove Structure"))
  (return (make `/Game/Blueprints/Gamemodes/Core/FPlayerMove` (`self.ForwardInput`) (`self.SteeringInput`) DeltaTime (`GameplayStatics.GetTimeSeconds`))))

(fn `GetLastMove`
  (returns (LastMove :type "/Game/Blueprints/Gamemodes/Core/FPlayerMove Structure"))
  (return (`self.LastMove`)))

(fn `GetVelocity`
  (returns (Velocity :type "Vector Structure"))
  (return (`self.Velocity`)))

(fn `SetSteeringInput`
  (params (SteeringInput :type "Float (double-precision)"))
  (set `self.SteeringInput` SteeringInput))

(fn `SetThrottleInput`
  (params (ThrottleInput :type "Float (double-precision)"))
  (set `self.ForwardInput` ThrottleInput))

(fn `SetVelocity`
  (params (Velocity :type "Vector Structure"))
  (set `self.Velocity` Velocity))

(fn `SimulateMove`
  (params (Move :type "/Game/Blueprints/Gamemodes/Core/FPlayerMove Structure (by ref)"))
  ;[1 1 1] Acceleration = Force / Mass
  (bind _output_get (set `self.Force` (+ (`self.CalculateAirResistance`) (`self.CalculateRollingResistance`) (* (`Actor.GetActorForwardVector` (`self.GetOwner`)) (`self.MaxForwardForce`) Move_ForwardInput_5_B9694660EF49BCCF5FFD75BC949DF323))))
  (bind _output_get_2 (set `self.Acceleration` (/ _output_get (`self.KartMass`))))
  ;[1 1 1] Velocity = Velocity + Acceleration * Time
  (set `self.Velocity` (+ (* _output_get_2 Move_DeltaTime_8_28020D0C6A4D0110B7740A942AFDF704) (`self.Velocity`)))
  ;[1 1 1] Update Location and Rotation
  (`self.ApplyRotation` Move_SteeringInput_6_C4E7A31C2A489A37B8EF2ABD6C5C5821 Move_DeltaTime_8_28020D0C6A4D0110B7740A942AFDF704)
  (`self.UpdateLocationFromVelocity` Move_DeltaTime_8_28020D0C6A4D0110B7740A942AFDF704))

(fn `UpdateLocationFromVelocity`
  (params (DeltaTime :type "Float (double-precision)"))
  ;[1 1 1] Offset = Velocity * 100 (m/s to cm/s) * Time
  (bind _sweephitresult (`Actor.K2_AddActorWorldOffset` (`self.GetOwner`) (* DeltaTime (`self.Velocity`) 100.0) true false)))