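; BP_SuspensionComponent is a suspension component that pushes its parent component away from the surface beneath it.
; InitComponent stores the parent, turns off its physics simulation and sets linear and angular damping.
; Each Tick traces down the component's local up axis over SuspensionLength.
; A hit applies force at the component's location along the impact normal, fading linearly from SuspensionForce to zero at full length.
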(event `InitComponent`
  (params (ParentComponent :type "StaticMeshComponent Object Reference"))
  (bind _parentcomponent (`self.ParentComponent`))
  (bind _output_get (set `self.ParentComponent` ParentComponent))
  (`PrimitiveComponent.SetSimulatePhysics` _output_get false)
  (`PrimitiveComponent.SetLinearDamping` _parentcomponent 3.0)
  (`PrimitiveComponent.SetAngularDamping` _parentcomponent 5.0))

(event `self.ReceiveTick`
  (params (DeltaSeconds :type "Float (single-precision)"))
  (bind _returnvalue (`self.K2_GetComponentLocation`))
  (bind (_outhit _returnvalue_2) (`KismetSystemLibrary.LineTraceSingle` _returnvalue (+ _returnvalue (* (`self.GetUpVector`) (`self.SuspensionLength`) -1.0)) "TraceTypeQuery1"))
  (if _returnvalue_2
    (bind (_bblockinghit _binitialoverlap _time _distance _location _impactpoint _normal _impactnormal) (`GameplayStatics.BreakHitResult` _outhit))
    (`PrimitiveComponent.AddForceAtLocation` (`self.ParentComponent`) (* _impactnormal (`KismetMathLibrary.Lerp` (`self.SuspensionForce`) 0.0 (/ (`KismetMathLibrary.VSize` (- _location (`self.K2_GetComponentLocation`))) (`self.SuspensionLength`)))) (`self.K2_GetComponentLocation`) "None")))