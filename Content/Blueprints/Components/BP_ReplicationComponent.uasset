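; Replication component that networks its owner's custom movement through client prediction and server reconciliation, working with BP_MovementComponent.
; Each tick the autonomous proxy queues and sends its last move, while simulated proxies replay the last replicated move.
; The server simulates received moves, with validation stubbed to always pass, and publishes move, velocity and transform as ServerState.
; On replication, clients snap to ServerState, discard acknowledged moves and replay the rest.
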(event `self.ReceiveBeginPlay`
  (set `self.MovementComponent` (`Actor.GetComponentByClass` (`self.GetOwner`) "/Game/Blueprints/Components/BP_MovementComponent.BP_MovementComponent_C")))

(event `self.ReceiveTick`
  (params (DeltaSeconds :type "Float (single-precision)"))
  (bind _serverstate_lastplayermove (break `/Game/Blueprints/Gamemodes/Core/FPlayerMoveState` (`self.ServerState`)))
  (bind _movementcomponent (`self.MovementComponent`))
  (`|ExecutionSequence`
    (:`then_0`
      ;[1 1 1] Simulates The Player on Local Machine
      (if (`|EnumEquality` (`Actor.GetLocalRole` (`self.GetOwner`)) "ROLE_AutonomousProxy")
        (bind _lastmove (`/Game/Blueprints/Components/BP_MovementComponent.GetLastMove` _movementcomponent))
        (`KismetArrayLibrary.Array_Add` (`self.UnacknowledgedMoves`) _lastmove)
        (`self.Server_SendMove` _lastmove)))
    (:`then_1`
      ;[1 1 1] Updates Server State
      (if (`|EnumEquality` (`Actor.GetRemoteRole` (`self.GetOwner`)) "ROLE_SimulatedProxy")
        (bind _lastmove_2 (`/Game/Blueprints/Components/BP_MovementComponent.GetLastMove` _movementcomponent))
        (`self.UpdateServerState` _lastmove_2)))
    (:`then_2`
      ;[1 1 1] Simulates Other Players On Local Machine
      (if (`|EnumEquality` (`Actor.GetLocalRole` (`self.GetOwner`)) "ROLE_SimulatedProxy")
        (`/Game/Blueprints/Components/BP_MovementComponent.SimulateMove` (`self.MovementComponent`) _serverstate_lastplayermove)))))

(event `Server_SendMove`
  (params (Move :type "/Game/Blueprints/Gamemodes/Core/FPlayerMove Structure"))
  ;[0.07998 1 0] RPC - Sends Move To The Server
  (if true
    (`/Game/Blueprints/Components/BP_MovementComponent.SimulateMove` (`self.MovementComponent`) Move)
    (`self.UpdateServerState` Move)
    (else
      (`KismetSystemLibrary.PrintString` "Validation Error"))))

(fn `ClearAcknowledgedMoves`
  (params (LastMove :type "/Game/Blueprints/Gamemodes/Core/FPlayerMove Structure"))
  (locals (NewMoves :type "Array of /Game/Blueprints/Gamemodes/Core/FPlayerMove Structure"))
  (for _array_element (`self.UnacknowledgedMoves`)
    (if (> (`.Time_10_F3CC948B9F443D492C71B2A7C14C319D` (break `/Game/Blueprints/Gamemodes/Core/FPlayerMove` _array_element)) (`.Time_10_F3CC948B9F443D492C71B2A7C14C319D` (break `/Game/Blueprints/Gamemodes/Core/FPlayerMove` LastMove)))
      (`KismetArrayLibrary.Array_Add` (`local.NewMoves`) _array_element)))
  (set `self.UnacknowledgedMoves` (`local.NewMoves`)))

(fn `OnRep_ServerState`
  (bind (_serverstate_lastplayermove _serverstate_velocity _serverstate_transform) (break `/Game/Blueprints/Gamemodes/Core/FPlayerMoveState` (`self.ServerState`)))
  (bind _movementcomponent (`self.MovementComponent`))
  ;[1 1 1] When Client Gets Move Update Velocity and Transform
  (`/Engine/EditorBlueprintResources/StandardMacros.IsValid` _movementcomponent
    (:`Is Valid`
      (`/Game/Blueprints/Components/BP_MovementComponent.SetVelocity` _movementcomponent _serverstate_velocity)
      (`Actor.K2_SetActorTransform` (`self.GetOwner`) _serverstate_transform false false)
      (`self.ClearAcknowledgedMoves` _serverstate_lastplayermove)
      (for _array_element (`self.UnacknowledgedMoves`)
        (`/Game/Blueprints/Components/BP_MovementComponent.SimulateMove` (`self.MovementComponent`) _array_element)))))

(fn `UpdateServerState`
  (params (Move :type "/Game/Blueprints/Gamemodes/Core/FPlayerMove Structure (by ref)"))
  (bind _velocity (`/Game/Blueprints/Components/BP_MovementComponent.GetVelocity` (`self.MovementComponent`)))
  (set `self.ServerState` (make `/Game/Blueprints/Gamemodes/Core/FPlayerMoveState` Move _velocity (`Actor.GetTransform` (`self.GetOwner`)))))